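; Front door Blueprint that serves as a key-locked exit, ending the level and returning the player to the main menu.
; On Interact, IsKey casts the player to FirstPersonCharacter and checks its KeyList for the door's Id.
; With a matching key, it plays the FadeOut level sequence, waits briefly, then opens the mainMenu level.
; Without the key, interaction does nothing.
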(event EventBeginPlay)

(event Collision|EventActorBeginOverlap
  (params (OtherActor :type Actor%20Object%20Reference)))

(event EventTick
  (params (DeltaSeconds :type Float%20%28single-precision%29)))

(event EventInteract
  (bind _key_present (CallFunction|IsKey))
  (if _key_present
    ;[1 1 1] Exit Code
    (bind _returnvalue (Sequencer|Player|CreateLevelSequencePlayer "/Game/Sequences/FadeOut.FadeOut"))
    (Sequencer|Player|Play _returnvalue :!class /Script/MovieScene.MovieSceneSequencePlayer)
    (Utilities|FlowControl|Delay 2.0)
    (Game|OpenLevel(byName) "mainMenu")))

(fn ConstructionScript)

(fn IsKey
  (bind _asfirst_person_character (Utilities|Casting|CastToFirstPersonCharacter (Game|GetPlayerCharacter 0)))
  (return (not (== (Utilities|Array|FindItem (Variables|/Game/FirstPersonBP/Blueprints/FirstPersonCharacter.FirstPersonCharacter_C|Getkey_list _asfirst_person_character) (Variables|Default|Getid)) -1))))